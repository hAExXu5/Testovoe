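; Elevator actor that moves vertically to a requested floor.
; Transport stores the target floor, picks up or down by comparing it with Current, and flags movement.
; Tick applies a fixed, frame-rate-dependent Z offset without sweep until height exactly equals the target's entry in Positions.
; Current is never updated in these graphs, and a travel time and velocity calculation is left unconnected.
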(event Custom|Transport
  (params (Floor :type Integer))
  (Variables|Default|SetDuringMovement true)
  (bind _output_get (Variables|Default|SetTarget Floor))
  (if (>= _output_get (Variables|Default|GetCurrent))
    (Variables|Default|SetDirection 1.0)
    (else
      (Variables|Default|SetDirection -1.0))))

(event EventTick
  (params (DeltaSeconds :type Float%20%28single-precision%29))
  (if (== (.z (Transformation|GetActorLocation)) (Utilities|Array|Get(acopy) (Variables|Default|GetPositions) (Variables|Default|GetTarget)))
    (bind _output_get (Variables|Default|SetDuringMovement false))
    (elif _output_get
      (Transformation|AddActorLocalOffset (* "0, 0,3.000000" (Variables|Default|GetDirection)) false false))))

(fn ConstructionScript)